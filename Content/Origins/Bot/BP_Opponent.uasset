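; BP_Opponent is a bot pawn that follows the ball, a BP_OrignsProjectile, along the X axis.
; Each Tick, it sets FloatingPawnMovement velocity to full speed toward the ball, stopping when their absolute X values are within a fixed dead zone.
; GetBall caches the projectile and looks it up again by class when the reference is invalid.
; A looping AdjustPosition timer starts on BeginPlay, but its event is empty.
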(event `self.ReceiveBeginPlay`
  (`KismetSystemLibrary.K2_SetTimerDelegate` (delegate `Adjust Position`) 0.1 true))

(event `Adjust Position`)

(event `self.ReceiveTick`
  (params (DeltaSeconds :type "Float (single-precision)"))
  (bind _returnvalue_x (`KismetMathLibrary.BreakVector` (`self.K2_GetActorLocation`)))
  (bind _floatingpawnmovement (`self.FloatingPawnMovement`))
  (bind _max_speed (`self.Max Speed`))
  (bind _returnvalue_x_2 (`KismetMathLibrary.BreakVector` (`SceneComponent.K2_GetComponentLocation` (`/Game/Origins/Projectile/BP_OrignsProjectile.Sphere` (`self.Ball`)))))
  (`/Engine/EditorBlueprintResources/StandardMacros.IsValid` (`self.Get Ball`)
    (:`Is Valid`
      (if (> (`KismetMathLibrary.Abs` (- (`KismetMathLibrary.Abs` _returnvalue_x_2) (`KismetMathLibrary.Abs` _returnvalue_x))) 55.0)
        (set `MovementComponent.Velocity` (`KismetMathLibrary.SelectVector` (`KismetMathLibrary.MakeVector` _max_speed) (`KismetMathLibrary.MakeVector` (* _max_speed -1.0)) (> _returnvalue_x_2 _returnvalue_x)) _floatingpawnmovement)
        (else
          (set `MovementComponent.Velocity` (0.0 0.0 0.0) _floatingpawnmovement))))))

(fn `Get Ball`
  (returns (Ball :type "/Game/Origins/Projectile/BP_OrignsProjectile Object Reference"))
  (bind _ball (`self.Ball`)
    (:`then`
      (return _ball))
    (:`else`
      (bind _returnvalue (`GameplayStatics.GetActorOfClass` "/Game/Origins/Projectile/BP_OrignsProjectile.BP_OrignsProjectile_C"))
      (bind _output_get (set `self.Ball` _returnvalue))
      (return _output_get))))

(fn `UserConstructionScript`)