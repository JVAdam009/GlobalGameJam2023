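; Player controller for the Origins mode that handles the pause menu and the game over screen.
; The Pause input checks the game's paused state to either create a new pause widget or remove it, switching pause, input mode and cursor to match.
; ShowGameOverScreen creates WBP_GameOverMenu with the PlayerWon result, then pauses the game and enables UI input with the cursor.
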(event `InputAction|Pause`
  (params (Key :type "Key Structure"))
  (bind _returnvalue (`GameplayStatics.GetPlayerController` 0))
  (bind _returnvalue_2 (`GameplayStatics.GetPlayerController` 0))
  ;[1 0.2048 0.9189] Pause Menu
  (:`Pressed`
    (if (`GameplayStatics.IsGamePaused`)
      (`Widget.RemoveFromParent` (stale _returnvalue_3))
      (`WidgetBlueprintLibrary.SetInputMode_GameOnly` _returnvalue)
      (set `PlayerController.bShowMouseCursor` false _returnvalue)
      (`GameplayStatics.SetGamePaused` false)
      (else
        (bind _returnvalue_3 (`|CreateWidget` "/Game/UI/Pausemenu.Pausemenu_C"))
        (`UserWidget.AddToViewport` _returnvalue_3 0)
        (`GameplayStatics.SetGamePaused` true)
        (`WidgetBlueprintLibrary.SetInputMode_GameAndUIEx` _returnvalue_2 null)
        (set `PlayerController.bShowMouseCursor` true _returnvalue_2)))))

(event `Show Game Over Screen`
  (params (`Player Won?` :type Boolean))
  (bind _returnvalue (`GameplayStatics.GetPlayerController` 0))
  (bind _returnvalue_2 (`|CreateWidget` "/Game/UI/WBP_GameOverMenu.WBP_GameOverMenu_C" null `Player Won?`))
  (`UserWidget.AddToViewport` _returnvalue_2 0)
  (`GameplayStatics.SetGamePaused` true)
  (`WidgetBlueprintLibrary.SetInputMode_GameAndUIEx` _returnvalue null)
  (set `PlayerController.bShowMouseCursor` true _returnvalue))

(fn `UserConstructionScript`)