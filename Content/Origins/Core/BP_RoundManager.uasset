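; Round manager actor for a player-versus-bot ball game that runs rounds, tracks both scores and handles restarts.
; On BeginPlay it creates the player HUD, then each round spawns a projectile ball at a center offset, broadcasts it through OriginsPlayerSubsystem and plays a start sound.
; Scoring updates the HUD and either starts a new round or, at MaxScore, shows the game over screen through the player controller.
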(event `self.ReceiveBeginPlay`
  (bind _returnvalue (`|CreateWidget` "/Game/UI/PlayerHUD/WBP_PlayerHUD.WBP_PlayerHUD_C"))
  (bind _output_get (set `self.(UI) Player HUD` _returnvalue))
  (`UserWidget.AddToViewport` _output_get 0)
  (`self.Start Round`))

(event `Start Round`
  (bind _returnvalue (+ (`self.Center Location`) (`self.K2_GetActorLocation`)))
  (bind _returnvalue_2 (`|SpawnActorFromClass` "/Game/Origins/Projectile/BP_OrignsProjectile.BP_OrignsProjectile_C" (`KismetMathLibrary.MakeTransform` _returnvalue) "Undefined" "OverrideRootScale" null null))
  (`OriginsPlayerSubsystem.BroadcastBallSpawned` (pcsubsystem `OriginsPlayerSubsystem` (`GameplayStatics.GetPlayerController` 0)) _returnvalue_2)
  (`GameplayStatics.PlaySoundAtLocation` "/Game/Origins/Sounds/Origin_GameStart_01.Origin_GameStart_01" _returnvalue (struct) 1.0 1.0 0.0 null null null null))

(fn `Increment Score`
  (params (Side :type "/Game/Origins/Triggers/ESide Enum" :default "NewEnumerator0"))
  (switch `/Game/Origins/Triggers/ESide` Side
    (:`NewEnumerator0`
      (bind _result (`/Engine/EditorBlueprintResources/StandardMacros.IncrementInt` (`self.Score - Player`))
        (:`  `
          (`/Game/UI/PlayerHUD/WBP_ScoreScreen.Set Score` (`/Game/UI/PlayerHUD/WBP_PlayerHUD.WBP_ScoreScreen` (`self.(UI) Player HUD`)) Side _result)
          (if (>= (`self.Score - Player`) (`self.Max Score`))
            (bind _asbp_origins_player_controller (cast `/Game/Origins/Character/BP_OriginsPlayerController` (`GameplayStatics.GetPlayerController` 0)))
            (`/Game/Origins/Character/BP_OriginsPlayerController.Show Game Over Screen` _asbp_origins_player_controller true)
            (else
              (`self.Start Round`))))))
    (:`NewEnumerator1`
      (bind _result_2 (`/Engine/EditorBlueprintResources/StandardMacros.IncrementInt` (`self.Score - Bot`))
        (:`  `
          (`/Game/UI/PlayerHUD/WBP_ScoreScreen.Set Score` (`/Game/UI/PlayerHUD/WBP_PlayerHUD.WBP_ScoreScreen` (`self.(UI) Player HUD`)) Side _result_2)
          (if (>= (`self.Score - Bot`) (`self.Max Score`))
            (bind _asbp_origins_player_controller_2 (cast `/Game/Origins/Character/BP_OriginsPlayerController` (`GameplayStatics.GetPlayerController` 0)))
            (`/Game/Origins/Character/BP_OriginsPlayerController.Show Game Over Screen` _asbp_origins_player_controller_2 false)
            (else
              (`self.Start Round`))))))))

(fn `Restart Game`
  (set `self.Score - Player` 0)
  (set `self.Score - Bot` 0)
  (`/Game/UI/PlayerHUD/WBP_PlayerHUD.Game Restarted` (`self.(UI) Player HUD`))
  (`self.Start Round`))

(fn `UserConstructionScript`)