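; BP_GravityObstacle is an obstacle that tracks the player's ball, with no gravity force applied in its graphs.
; On BeginPlay it binds to the ball-spawned event of OriginsPlayerSubsystem and stores each newly spawned ball.
; While that ball is valid, Tick prints the unit direction from the obstacle to the ball as debug output.
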(event `self.ReceiveBeginPlay`
  (add `OriginsPlayerSubsystem.OnBallSpawned` (pcsubsystem `OriginsPlayerSubsystem` (`GameplayStatics.GetPlayerController` 0)) (delegate `New Ball Spawned`)))

(event `New Ball Spawned`
  (params (Ball :type "OriginsProjectile Object Reference"))
  (set `self.Ball` Ball))

(event `self.ReceiveTick`
  (params (DeltaSeconds :type "Float (single-precision)"))
  (bind _ball (`self.Ball`)
    (:`then`
      (`KismetSystemLibrary.PrintString` (`KismetStringLibrary.Concat_StrStr` "Direction: " (`KismetStringLibrary.Conv_VectorToString` (`KismetMathLibrary.GetDirectionUnitVector` (`self.K2_GetActorLocation`) (`self.K2_GetActorLocation` _ball))))))
    (:`else`)))

(fn `UserConstructionScript`)