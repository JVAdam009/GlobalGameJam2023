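; Physics-driven ball projectile that players hit, with bounce sounds and a destroy broadcast to the player subsystem.
; Tick clamps velocity, enforces a minimum Y speed once a character has hit it, and plays a sound on sharp X/Y velocity changes.
; A looping timer applies counter-impulses against upward Z motion.
; A hit handler, not called here, optionally boosts X/Y using the character's forward vector, with Y forced positive.
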(event `self.ReceiveBeginPlay`
  ;[0.01042 0.01042 0.01042] Begin Play
  (`KismetSystemLibrary.K2_SetTimer` null "Limit Z Climb" 0.5 true))

(event `self.Sphere.OnComponentHit`
  (params (HitComponent :type "PrimitiveComponent Object Reference") (OtherActor :type "Actor Object Reference") (OtherComp :type "PrimitiveComponent Object Reference") (NormalImpulse :type "Vector Structure") (Hit :type "HitResult Structure (by ref)"))
  ;[0.01042 0.01042 0.01042] On Hit
  (`GameplayStatics.PlaySoundAtLocation` "/Game/Origins/Sounds/SC_BallHit.SC_BallHit" (`self.K2_GetActorLocation`) (struct) 1.0 1.0 0.0 null null null null)
  (cast `/Game/Origins/Character/BP_OriginsCharacter` OtherActor)
  (set `self.Has Been Hit By Player?` true))

(event `self.ReceiveTick`
  (params (DeltaSeconds :type "Float (single-precision)"))
  (bind _sphere (`self.Sphere`))
  (bind (_old_velocity_x _old_velocity_y) (`KismetMathLibrary.BreakVector` (`self.Old Velocity`)))
  ;[0.01042 0.01042 0.01042] Tick
  (`|ExecutionSequence`
    (:`then_0`
      ;;[0.01042 0.01042 0.01042] Clamp Velocity
      (bind _returnvalue (`PrimitiveComponent.GetPhysicsLinearVelocity` _sphere "None"))
      (bind _out_velocity (`self.Clamp Velocity` _returnvalue))
      (if (`self.Has Been Hit By Player?`)
        (bind _out_velocity_2 (`self.Ensure Min Velocity` _out_velocity))
        (`PrimitiveComponent.SetPhysicsLinearVelocity` _sphere _out_velocity_2 false "None")
        (else
          (`PrimitiveComponent.SetPhysicsLinearVelocity` _sphere _out_velocity false "None"))))
    (:`then_1`
      ;;[0.01042 0.01042 0.01042] Play Sound On Direction Change
      (bind _returnvalue_2 (`PrimitiveComponent.GetPhysicsLinearVelocity` _sphere "None"))
      (if (or (> (`KismetMathLibrary.Abs` (- (.x _returnvalue_2) _old_velocity_x)) 300.0) (> (`KismetMathLibrary.Abs` (- (.y _returnvalue_2) _old_velocity_y)) 300.0))
        (`GameplayStatics.PlaySoundAtLocation` "/Game/Origins/Sounds/SC_BallHit.SC_BallHit" (`self.K2_GetActorLocation`) (struct) 1.0 1.0 0.0 null null null null)))
    (:`then_2`
      ;;[0.01042 0.01042 0.01042] Save Velocity for Comparison on Next Tick
      (bind _returnvalue_3 (`PrimitiveComponent.GetPhysicsLinearVelocity` (`self.Sphere`) "None"))
      (bind _output_get (set `self.Old Velocity` _returnvalue_3))
      (`KismetSystemLibrary.PrintString` (`KismetStringLibrary.Concat_StrStr` "Velocity: " (`KismetStringLibrary.Conv_VectorToString` _output_get)) true true (struct :`R` 1.0 :`G` 0.979058 :`B` 0.121041 :`A` 1.0) 0.0))))

(fn `Destroy Ball`
  (`OriginsPlayerSubsystem.BroadcastBallDestroyed` (pcsubsystem `OriginsPlayerSubsystem` (`GameplayStatics.GetPlayerController` 0)) self)
  (`self.K2_DestroyActor`))

(fn `Handle Player Hitting Ball`
  (params (Character :type "/Game/Origins/Character/BP_OriginsCharacter Object Reference"))
  (locals (`(L) Boost` :type "Vector Structure") (`(L) Should Boost?` :type Boolean))
  (bind (_returnvalue_x _returnvalue_y) (`KismetMathLibrary.BreakVector` (`self.GetVelocity`)))
  (bind (_boost_force_x _boost_force_y) (`KismetMathLibrary.BreakVector` (`self.Boost Force`)))
  (bind _boost_force_x_2 (`KismetMathLibrary.BreakVector` (`self.Boost Force`)))
  (bind (_returnvalue_x_2 _returnvalue_y_2 _returnvalue_z) (`KismetMathLibrary.BreakVector` (`SceneComponent.GetForwardVector` (`Character.CapsuleComponent` Character))))
  (bind _returnvalue (* (`KismetMathLibrary.MakeVector` _returnvalue_x_2 (`KismetMathLibrary.Abs` _returnvalue_y_2) _returnvalue_z) (`local.(L) Boost`)))
  (`|ExecutionSequence`
    (:`then_1`
      (`|ExecutionSequence`
        (:`then_0`
          ;[0.02083 0.02083 0.02083] Set X Impulse
          (if (`self.Boost X?`)
            (if (or (< (`KismetMathLibrary.Abs` _returnvalue_x) (`self.Min Boost Speed`)) (== (`self.Min Boost Speed`) 0.0))
              (set `local.(L) Boost` (+ (`local.(L) Boost`) (`KismetMathLibrary.MakeVector` _boost_force_x_2)))
              (set `local.(L) Should Boost?` true))))
        (:`then_1`
          ;[0.02083 0.02083 0.02083] Set Y Impulse
          (if (`self.Boost Y?`)
            (if (or (< (`KismetMathLibrary.Abs` _returnvalue_y) (`self.Min Boost Speed`)) (== (`self.Min Boost Speed`) 0.0))
              (set `local.(L) Boost` (+ (`local.(L) Boost`) (`KismetMathLibrary.MakeVector` 0.0 _boost_force_y)))
              (set `local.(L) Should Boost?` true))))
        (:`then_2`
          ;[0.02083 0.02083 0.02083] Boost
          (if (`local.(L) Should Boost?`)
            (`PrimitiveComponent.AddImpulse` (`self.Sphere`) _returnvalue "None" true)
            (`KismetSystemLibrary.PrintString` (`KismetStringLibrary.Concat_StrStr` "BOOST: " (`KismetStringLibrary.Conv_VectorToString` _returnvalue)))))))))

(fn `Limit Z Climb`
  (bind _returnvalue (`PrimitiveComponent.GetPhysicsLinearVelocity` (`self.Sphere`) "None"))
  (if (> (.z _returnvalue) 0.0)
    (`PrimitiveComponent.AddImpulse` (`self.Sphere`) (`KismetMathLibrary.MakeVector` 0.0 0.0 (* (.z _returnvalue) -1.0)) "None" false)))

(fn `UserConstructionScript`)